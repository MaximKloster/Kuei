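; A wall that BP_Optimized_Drag_Charakter cannot pass through, with configurable visibility.
; The construction script stretches, centers and rotates the wall mesh from the actor origin to EndPoint at the set height.
; On collision overlap it notifies the character, and Tick pins the capsule to the stored non-collided position until overlap ends.
; End overlap saves the capsule's current location as that safe position.
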(event `self.ReceiveBeginPlay`)

(event `self.ReceiveActorBeginOverlap`
  (params (OtherActor :type "Actor Object Reference")))

(event `self.ReceiveTick`
  (params (DeltaSeconds :type "Float (single-precision)"))
  (if (`self.CharakterCollided`)
    (`SceneComponent.K2_SetWorldLocation` (`Character.CapsuleComponent` (`self.Charakter`)) (`self.NoCollisionPoint`) false)))

(event `self.Collision.OnComponentBeginOverlap`
  (params (OtherActor :type "Actor Object Reference") (OtherComp :type "PrimitiveComponent Object Reference") (OtherBodyIndex :type Integer) (bFromSweep :type Boolean) (SweepResult :type "HitResult Structure (by ref)"))
  (bind _asbp_optimized_drag_charakter (cast `/Game/Blueprints/BP_Optimized_Drag_Charakter` OtherActor))
  (set `self.Charakter` _asbp_optimized_drag_charakter)
  (set `self.CharakterCollided` true)
  (set `self.NoCollisionPoint` (`/Game/Blueprints/BP_Optimized_Drag_Charakter.NotCollidedPosition` _asbp_optimized_drag_charakter))
  (`/Game/Blueprints/BP_Optimized_Drag_Charakter.InNotMoveableWall` _asbp_optimized_drag_charakter))

(event `self.Collision.OnComponentEndOverlap`
  (params (OtherActor :type "Actor Object Reference") (OtherComp :type "PrimitiveComponent Object Reference") (OtherBodyIndex :type Integer))
  (bind _asbp_optimized_drag_charakter (cast `/Game/Blueprints/BP_Optimized_Drag_Charakter` OtherActor))
  (set `self.CharakterCollided` false)
  (set `/Game/Blueprints/BP_Optimized_Drag_Charakter.NotCollidedPosition` (`SceneComponent.K2_GetComponentLocation` (`Character.CapsuleComponent` _asbp_optimized_drag_charakter)) _asbp_optimized_drag_charakter))

(fn `UserConstructionScript`
  (bind _returnvalue (`self.K2_GetActorLocation`))
  (bind _wallhight (`self.WallHight`))
  (bind _endpoint (`self.EndPoint`))
  (bind _wall (`self.Wall`))
  (`SceneComponent.SetVisibility` _wall (`self.Visibil`) false)
  (if (!= _endpoint (0.0 0.0 0.0))
    (`SceneComponent.SetWorldScale3D` _wall (`KismetMathLibrary.MakeVector` (/ (`KismetMathLibrary.VSize` _endpoint) 256.0) 0.05 (/ _wallhight 256.0)))
    (`SceneComponent.K2_SetRelativeLocation` _wall (`KismetMathLibrary.MakeVector` (/ (.x _endpoint) 2.0) (/ (.y _endpoint) 2.0) (/ _wallhight 2.0)) false)
    (`SceneComponent.K2_SetWorldRotation` _wall (`KismetMathLibrary.MakeRot` 0.0 (.yaw (`KismetMathLibrary.FindLookAtRotation` _returnvalue (+ _endpoint _returnvalue)))) false)))